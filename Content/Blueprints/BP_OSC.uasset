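; BP_OSC is a Blueprint that receives acceleration data over OSC and stores it as AccelX.
; On BeginPlay it starts an OSC server on a hardcoded IP and port and binds to its message-received event.
; OSCIn switches on the last segment of each message address; for Accel, it keeps the magnitude of the first float when below a negative threshold, otherwise zero.
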(event Custom|OSCIn
  (params (Message :type OSC%20Message%20Structure%20%28by%20ref%29) (IPAddress :type String) (Port :type Integer))
  (bind _output_get (Variables|Default|SetOSCMessage Message))
  (bind _returnvalue (Class|OSCManager|GetOSCMessageAddress _output_get))
  (bind _returnvalue_2 (Class|OSCManager|GetOSCAddressFullPath _returnvalue))
  (switch string (.RightS (Utilities|String|Split _returnvalue_2 "/" "IgnoreCase" "FromEnd"))
    (:accel
      (bind _value (Class|OSCManager|GetFloat (Variables|Default|GetOSCMessage)))
      (if (< _value -0.5)
        (Variables|Default|SetAccelX (Math|Float|Absolute(Float) _value))
        (else
          (Variables|Default|SetAccelX 0.0))))))

(event EventBeginPlay
  (bind _returnvalue (Class|OSCManager|CreateOSCServer "192.168.0.118" 50000 false true "" 0))
  (bind _output_get (Variables|Default|SetOSCServer _returnvalue))
  (EventDispatchers|BindEventtoOnOscMessageReceived _output_get (EventDispatchers|CreateEvent :!event Custom|OSCIn)))

(fn ConstructionScript)